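; Damage system component that tracks an actor's health, death, blocking, invincibility and interruptibility.
; TakeDamage routes a damage info struct through a CanBeDamaged macro to block, apply or ignore the hit.
; It fires dispatchers for blocks (with parry flag), death, and damage responses on interruptible or forced-interrupt hits.
; Heal restores a percentage of max health, clamped, while the owner is alive.
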(event EventBeginPlay)

(event EventTick
  (params (DeltaSeconds :type Float%20%28single-precision%29)))

(fn Heal
  (params (Amount :type Float%20%28double-precision%29))
  (if (not (Variables|Default|GetIsDead))
    (bind _output_get (Variables|Default|SetHealth (Math|Float|Clamp(Float) (+ (* (/ (Variables|Default|GetMaxHealth) 1e+02) Amount) (Variables|Default|GetHealth)) 0.0 (Variables|Default|GetMaxHealth))))
    (return _output_get)))

(fn TakeDamage
  (params (DamageInfo :type ST%20Damage%20Info%20Structure) (DamageCauser :type Actor%20Object%20Reference))
  (bind (_damageamount _damagetype _damageresponse _shoulddamageinvincible _canbeblocked _canbeparried _shouldforceintrerrupt) (Utilities|Struct|BreakST_DamageInfo DamageInfo))
  (Utilities|CanbeDamaged _shoulddamageinvincible _canbeblocked
    (:BlockDamage
      (Default|CallOnBlocked _canbeparried)
      (return false))
    (:DoDamage
      (bind _output_get (Variables|Default|SetHealth (- (Variables|Default|GetHealth) _damageamount)))
      (if (<= _output_get 0.0)
        (Variables|Default|SetIsDead true)
        (Default|CallOnDeath)
        (return true)
        (elif (or (Variables|Default|GetIsIntrerruptible) _shouldforceintrerrupt)
          (Default|CallOnDamageResponse _damageresponse DamageCauser)
          (return true))))
    (:NoDamage
      (return false))))