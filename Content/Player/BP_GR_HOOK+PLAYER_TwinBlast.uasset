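; TwinBlast player character Blueprint that handles throwing a grappling hook from the Enhanced Input grapple action.
; A throw requires a valid, in-range grapple point other than the current one, and launches the character toward the previous destination if already grappling.
; It then sets the destination above the point's landing zone, turns to face it, records rope length, marks the point used and plays an air or ground montage.
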(event Input|EnhancedActionEvents|EnhancedInputActionIA_Grapple
  (params (ActionValue :type Boolean) (ElapsedSeconds :type Float%20%28double-precision%29) (TriggeredSeconds :type Float%20%28double-precision%29) (InputAction :type Input%20Action%20Object%20Reference :default "/Game/ThirdPerson/Input/Actions/IA_Grapple.IA_Grapple"))
  (bind _mesh (Variables|Character|GetMesh))
  (bind _returnvalue (Components|SkeletalMesh|GetAnimInstance _mesh))
  ;[1 1 1] Throws the grappling hook
  (:Started
    (Utilities|IsValid (Variables|Default|GetGrapplePointRef)
      (:Is%20Valid
        (if (and (<= (Math|Vector|VectorLength (- (Transformation|GetActorLocation) (Transformation|GetActorLocation (Variables|Default|GetGrapplePointRef)))) (Variables|Default|GetGrappleThrowDistance)) (!= (Variables|Default|GetCurrentGrapplePoint) (Variables|Default|GetGrapplePointRef)))
          (if (Variables|Default|GetbMovingWithGrapple)
            (Character|LaunchCharacter (* (Math|Vector|GetUnitDirection(Vector) (Transformation|GetActorLocation) (Variables|Default|GetGrapplingDestination)) 2e+02) false false))
          (Variables|Default|SetbInGrapplingAnimation true)
          (Variables|Default|SetbMovingWithGrapple false)
          (Variables|Default|SetCurrentGrapplePoint (Variables|Default|GetGrapplePointRef))
          (Variables|Default|SetGrapplingDestination (+ (Transformation|GetWorldLocation (Variables|/Game/GrapplingHook/Core/BP_GrapplePoint.BP_GrapplePoint_C|GetLandingZone (Variables|Default|GetCurrentGrapplePoint))) "0, 0,110.000000"))
          (Transformation|SetActorRotation (Math|Rotator|MakeRotator 0.0 0.0 (.yaw (Math|Rotator|FindLookatRotation (Transformation|GetActorLocation) (Variables|Default|GetGrapplingDestination)))))
          (Variables|Default|SetRopeBaseLength (Math|Vector|VectorLength (- (Transformation|GetActorLocation) (Variables|Default|GetGrapplingDestination))))
          (Default|Use (Variables|Default|GetCurrentGrapplePoint))
          (if (AI|Components|NavMovement|IsFalling (Variables|Character|GetCharacterMovement))
            (Animation|Montage|MontagePlay _returnvalue "/Game/Player/TwinBlast_Animations/AM_TwinBlast_GrappleAir.AM_TwinBlast_GrappleAir" 1.0 "Duration" 0.0 true)
            (else
              (Animation|Montage|MontagePlay _returnvalue "/Game/Player/TwinBlast_Animations/AM_TwinBlast_GrappleGround.AM_TwinBlast_GrappleGround" 1.0 "Duration" 0.0 true))))))))

(event EventBeginPlay
  (|CallParentFunction) ; This node is disabled and will not be called.\nDrag off pins to build functionality.
)

(event Collision|EventActorBeginOverlap
  (params (OtherActor :type Actor%20Object%20Reference)))

(event EventTick
  (params (DeltaSeconds :type Float%20%28single-precision%29))
  (|CallParentFunction DeltaSeconds) ; This node is disabled and will not be called.\nDrag off pins to build functionality.
)

(fn ConstructionScript
  (|CallParentFunction))