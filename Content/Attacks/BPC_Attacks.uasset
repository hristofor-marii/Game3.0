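; Attack component that gives its owner a hitscan bullet and a homing-capable dark energy spell.
; FireBullet line-traces for Pawns, while MagicSpell spawns BP_Projectile_DarkEnergy with a target and binds its impact event.
; Both send hits a TakeDamage message and report an AI damage event at the owner's location.
; Only spell impact fires OnAttackEnded; the node making the projectile ignore its owner is disconnected.
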(event Custom|MagicSpell
  (params (SpawnTransform :type Transform) (Target :type Actor%20Object%20Reference) (DamageInfo :type ST%20Damage%20Info%20Structure))
  (bind _returnvalue (Game|SpawnActorfromClass "/Game/Projectiles/BP_Projectile_DarkEnergy.BP_Projectile_DarkEnergy_C" SpawnTransform "Undefined" "MultiplyWithRoot" (Components|GetOwner) 1e+03 0.0 Target false 0))
  (EventDispatchers|AssignOnProjectileImpact _returnvalue (delegate Custom|OnProjectileImpact_Event))
  (Development|PrintString "IGNORE"))

(event Custom|FireBullet
  (params (Start :type Vector) (End :type Vector) (DamageInfo :type ST%20Damage%20Info%20Structure))
  (bind _returnvalue (Components|GetOwner))
  (bind (_outhit _returnvalue_2) (Collision|LineTraceForObjects Start End (Utilities|Array|MakeArray "ObjectTypeQuery3") false 0 "None"))
  (if _returnvalue_2
    (Class|BPIDamageable|TakeDamage(Message) (.HitActor (Collision|BreakHitResult _outhit)) DamageInfo (Components|GetOwner))
    (Class|AISenseDamage|ReportDamageEvent (.HitActor (Collision|BreakHitResult _outhit)) _returnvalue (.DamageAmount (Utilities|Struct|BreakST_DamageInfo DamageInfo)) (Transformation|GetActorLocation _returnvalue) "0, 0, 0" "None")))

(event Custom|OnProjectileImpact_Event
  (params (OtherActor :type Actor%20Object%20Reference) (Hit :type Hit%20Result%20Structure))
  (bind _returnvalue (Components|GetOwner))
  (Class|BPIDamageable|TakeDamage(Message) OtherActor (stale Custom|MagicSpell DamageInfo) _returnvalue)
  (Class|AISenseDamage|ReportDamageEvent OtherActor _returnvalue (.DamageAmount (Utilities|Struct|BreakST_DamageInfo (stale Custom|MagicSpell DamageInfo))) (Transformation|GetActorLocation (Components|GetOwner)) "0, 0, 0" "None")
  (Default|CallOnAttackEnded))

(event EventBeginPlay)

(event EventTick
  (params (DeltaSeconds :type Float%20%28single-precision%29)))