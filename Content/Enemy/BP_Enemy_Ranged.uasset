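; Ranged enemy character that wields a rifle and shoots at the target chosen by its AI controller.
; On BeginPlay it spawns a rifle and attaches it to a hand socket.
; Attack plays a firing montage whose notify fires a damaging bullet from the weapon toward the controller's attack target, then signals attack end on completion or interruption.
; Overrides supply movement speeds and ideal attack and defend ranges, while the patrol route returns nothing.
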(event EventAttack
  (Variables|Default|SetAttacking true)
  (bind _notifyname (Animation|Montage|PlayMontage (Variables|Character|GetMesh) "/Game/Enemy/Animations/Montages/AM_FiringRifle_UE_Montage.AM_FiringRifle_UE_Montage")
    (:OnCompleted
      (Default|CallOnAttackEnd :!label _label)
      (Variables|Default|SetAttacking false))
    (:OnInterrupted
      (goto _label))
    (:OnNotifyBegin
      (switch name _notifyname
        (:Fire
          (bind _asaic_enemy_base (Utilities|Casting|CastToAIC_Enemy_Base (AI|GetAIController self)))
          (bind _attack_target (Variables|/Game/Enemy/AI/AIC_Enemy_Base.AIC_Enemy_Base_C|GetAttack%20Target _asaic_enemy_base)
            (:then
              (Default|FireBullet (Variables|Default|GetBPC_Attacks) (Transformation|GetActorLocation (Variables|Default|GetWeaponActor)) (Transformation|GetActorLocation _attack_target) (Utilities|Struct|MakeST_DamageInfo 15.0 "NewEnumerator2" "NewEnumerator1" false true)))
            (:else)))))))

(event EventEquipWeapon
  (bind _returnvalue (Game|SpawnActorfromClass "/Game/Props/BP_Weapon_Riffle.BP_Weapon_Riffle_C" (Transformation|GetActorTransform) "Undefined" "MultiplyWithRoot" 0 0))
  (bind _output_get (Variables|Default|SetWeaponActor _returnvalue))
  (Transformation|AttachComponentToComponent _output_get (Variables|Character|GetMesh) "hand_r_RiffleSocket" "SnapToTarget" "SnapToTarget" "SnapToTarget" true)
  (Default|CallOnWeaponEquipped)
  (Variables|Default|SetIsWieldingWeapon true))

(event EventBeginPlay
  (|CallParentFunction)
  (CallFunction|EquipWeapon))

(fn ConstructionScript
  (|CallParentFunction))

(fn SetMovementSpeed
  (params (Speed :type E_MovementSpeed%20Enum :default "NewEnumerator0"))
  (bind _output_get (Variables|/Script/Engine.CharacterMovementComponent|SetMaxWalkSpeed (Variables|Character|GetCharacterMovement) (Utilities|Select :Index Speed :NewEnumerator0 0.0 :NewEnumerator1 2e+02 :NewEnumerator2 3e+02 :NewEnumerator3 5e+02 :NewEnumerator4 1e+02)))
  (return _output_get))

(fn GetIdealRange
  (return 6e+02 6e+02))

(fn GetPatrolRoute
  (return 0))