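; Melee enemy Blueprint that attacks, blocks, and draws or sheathes a sword, with each action driven by montages.
; Montage notifies time the forward sphere-trace hit, which forces interrupts, and the sword's socketed spawn or destruction.
; BPC_DamageSystem handles incoming damage and holds interruptible and blocking flags; its OnBlocked event switches to an impact montage.
; Dispatchers report action endings, and a blocking state stops that montage switch from ending the block early.
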(event OnBlocked(BPC_DamageSystem)
  (params (CanBeParried :type Boolean))
  ;[1 1 1] Blocking
  (Variables|Default|SetBlockingState "NewEnumerator2")
  (Animation|Montage|PlayMontage (Variables|Character|GetMesh) "/Game/Enemy/Animations/Montages/AM_SwordImpact_UE.AM_SwordImpact_UE"
    (:OnCompleted
      _)
    (:OnInterrupted
      _))
  (CallFunction|EndBlock))

(event Custom|StartBlock
  ;[1 1 1] Blocking
  (Components|Movement|StopMovementImmediately (Variables|Character|GetCharacterMovement))
  (Variables|/Game/DamageSystem/BPC_DamageSystem.BPC_DamageSystem_C|SetIsBlocking (Variables|Default|GetBPC_DamageSystem) true)
  (Variables|Default|SetBlockingState "NewEnumerator1")
  (Animation|Montage|PlayMontage (Variables|Character|GetMesh) "/Game/Enemy/Animations/AM_SwordBlocking_UE_Montage.AM_SwordBlocking_UE_Montage"
    (:OnCompleted
      (CallFunction|EndBlock :!label _label))
    (:OnInterrupted
      (if (Utilities|Enum|NotEqual(Enum) (Variables|Default|GetBlockingState) "NewEnumerator2")
        (goto _label)))))

(event Custom|EndBlock
  ;[1 1 1] Blocking
  (Variables|/Game/DamageSystem/BPC_DamageSystem.BPC_DamageSystem_C|SetIsBlocking (Variables|Default|GetBPC_DamageSystem) false)
  (Variables|Default|SetBlockingState "NewEnumerator0")
  (Default|CallOnBlockEnded))

(event EventEquipWeapon
  (bind _notifyname (Animation|Montage|PlayMontage (Variables|Character|GetMesh) "/Game/Enemy/Animations/Montages/AM_DrawSword_Montage.AM_DrawSword_Montage")
    (:OnCompleted
      (Default|CallOnWeaponEquipped))
    (:OnNotifyBegin
      (switch name _notifyname
        (:UnsheatSword
          (bind _returnvalue (Game|SpawnActorfromClass "/Game/Props/BP_Weapon_Sword.BP_Weapon_Sword_C" (Transformation|GetActorTransform) "Undefined" "MultiplyWithRoot" 0 0))
          (bind _output_get (Variables|Default|SetWeaponActor _returnvalue))
          (Transformation|AttachComponentToComponent _output_get (Variables|Character|GetMesh) "hand_r_SwordSocket" "SnapToTarget" "SnapToTarget" "SnapToTarget" true)
          (Variables|Default|SetIsWieldingWeapon true))))))

(event Collision|EventActorBeginOverlap
  (params (OtherActor :type Actor%20Object%20Reference)))

(event EventUnequipWeapon
  (bind _notifyname (Animation|Montage|PlayMontage (Variables|Character|GetMesh) "/Game/Enemy/Animations/Montages/AM_SheathingSword_Montage.AM_SheathingSword_Montage")
    (:OnCompleted
      (Default|CallOnWeaponUnequipped :!label _label))
    (:OnInterrupted
      (goto _label))
    (:OnNotifyBegin
      (switch name _notifyname
        (:SheatSword
          (Actor|DestroyActor (Variables|Default|GetWeaponActor))
          (Variables|Default|SetIsWieldingWeapon false))))))

(event EventBeginPlay
  (|CallParentFunction)
  (Variables|Default|SetRootLocation (.location (Transformation|GetBoneTransform (Variables|Character|GetMesh) "root" "RTS_World"))))

(event EventTick
  (params (DeltaSeconds :type Float%20%28single-precision%29)))

(event EventAttack
  (bind _returnvalue (Transformation|GetActorLocation))
  (bind _notifyname (Animation|Montage|PlayMontage (Variables|Character|GetMesh) "/Game/Enemy/Animations/Montages/AM_Attack_Downward_Montage.AM_Attack_Downward_Montage")
    (:then
      (Variables|/Game/DamageSystem/BPC_DamageSystem.BPC_DamageSystem_C|SetIsIntrerruptible (Variables|Default|GetBPC_DamageSystem) false))
    (:OnCompleted
      (Default|CallOnAttackEnd :!label _label)
      (Variables|/Game/DamageSystem/BPC_DamageSystem.BPC_DamageSystem_C|SetIsIntrerruptible (Variables|Default|GetBPC_DamageSystem) true))
    (:OnInterrupted
      (goto _label))
    (:OnNotifyBegin
      (switch name _notifyname
        (:Slash
          (bind (_outhit _returnvalue_2) (Collision|SphereTraceForObjects _returnvalue (+ (* (Transformation|GetActorForwardVector) 2e+02) _returnvalue) 2e+01 (Utilities|Array|MakeArray "ObjectTypeQuery3") false 0 "ForDuration"))
          (if _returnvalue_2
            (Class|BPIDamageable|TakeDamage(Message) (.HitActor (Collision|BreakHitResult _outhit)) (Utilities|Struct|MakeST_DamageInfo 3e+01 "NewEnumerator1" "NewEnumerator0" false false false true) self)))))))

(fn ConstructionScript
  (|CallParentFunction))

(fn TakeDamage
  (params (DamageInfo :type ST%20Damage%20Info%20Structure) (Damage%20Causer :type Actor%20Object%20Reference))
  (bind _wasdamaged (Default|TakeDamage (Variables|Default|GetBPC_DamageSystem) DamageInfo Damage%20Causer))
  (return _wasdamaged))