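; BP_PatrolRoute is a patrol path actor that supplies spline points as waypoints for enemy AI.
; IncrementPatrolRoute steps PatrolIndex along the PatrolRoute spline, with SetDirection reversing at the first and last points for back-and-forth movement.
; GetSplinePointAsWorldPosition returns the current point's world location, and each increment also prints the direction for debugging.
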(event Custom|IncrementPatrolRoute
  (CallFunction|SetDirection)
  (Development|PrintString "Direction")
  (Development|PrintString (Utilities|String|ToString(Integer) (Variables|Default|GetDirection)))
  (Variables|Default|SetPatrolIndex (+ (Variables|Default|GetPatrolIndex) (Variables|Default|GetDirection))))

(event Custom|SetDirection
  ;[1 1 1] Aleg in ce directie sa ma misc
  (if (== (Variables|Default|GetPatrolIndex) 0)
    (Variables|Default|SetDirection 1)
    (elif (== (Variables|Default|GetPatrolIndex) (- (Spline|GetNumberOfSplinePoints (Variables|Default|GetPatrolRoute)) 1))
      (Variables|Default|SetDirection -1))))

(fn ConstructionScript)

(fn GetSplinePointasWorldPosition
  (return (Spline|GetLocationatSplinePoint (Variables|Default|GetPatrolRoute) (Variables|Default|GetPatrolIndex) "World")))