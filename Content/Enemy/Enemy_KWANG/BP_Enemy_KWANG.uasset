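; Sword-wielding KWANG enemy, a child Blueprint that turns off its AI controller's perception on BeginPlay.
; Montage notifies time spawning and attaching the sword, destroying it on sheathing, and a forward sphere-trace attack that deals interrupt-forcing damage.
; The damage system component holds health, interruptibility and blocking, with a blocked hit switching the block montage to an impact reaction.
; Equip, unequip, attack and block report their completion through event dispatchers.
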(event OnBlocked(BPC_DamageSystem)
  (params (CanBeParried :type Boolean))
  ;[1 1 1] Blocking
  (Variables|Default|SetBlockingState "NewEnumerator2")
  (Animation|Montage|PlayMontage (Variables|Character|GetMesh) "/Game/Enemy/Enemy_KWANG/Animations/AM_KWANGSwordImpact_UE.AM_KWANGSwordImpact_UE"
    (:OnCompleted
      _)
    (:OnInterrupted
      _))
  (CallFunction|EndBlock))

(event Custom|CustomEvent
  ;[1 1 1] Blocking
  (Components|Movement|StopMovementImmediately (Variables|Character|GetCharacterMovement))
  (Variables|/Game/DamageSystem/BPC_DamageSystem.BPC_DamageSystem_C|SetIsBlocking (Variables|Default|GetBPC_DamageSystem) true)
  (Variables|Default|SetBlockingState "NewEnumerator1")
  (Animation|Montage|PlayMontage (Variables|Character|GetMesh) "/Game/Enemy/Enemy_KWANG/Animations/AM_KWANGSwordBlocking_UE_Montage.AM_KWANGSwordBlocking_UE_Montage"
    (:OnCompleted
      (CallFunction|EndBlock :!label _label))
    (:OnInterrupted
      (if (Utilities|Enum|NotEqual(Enum) (Variables|Default|GetBlockingState) "NewEnumerator2")
        (goto _label)))))

(event Custom|CustomEvent_1
  ;[1 1 1] Blocking
  (Variables|/Game/DamageSystem/BPC_DamageSystem.BPC_DamageSystem_C|SetIsBlocking (Variables|Default|GetBPC_DamageSystem) false)
  (Variables|Default|SetBlockingState "NewEnumerator0")
  (Default|CallOnBlockEnded))

(event EventEquipWeapon
  (bind _notifyname (Animation|Montage|PlayMontage (Variables|Character|GetMesh) "/Game/Enemy/Enemy_KWANG/Animations/AM_KWANGDrawSword_Montage.AM_KWANGDrawSword_Montage")
    (:OnCompleted
      (Default|CallOnWeaponEquipped))
    (:OnNotifyBegin
      (switch name _notifyname
        (:UnsheatSword
          (bind _returnvalue (Game|SpawnActorfromClass "/Game/Props/BP_Weapon_Sword.BP_Weapon_Sword_C" (Transformation|GetActorTransform) "Undefined" "MultiplyWithRoot" 0 0))
          (bind _output_get (Variables|Default|SetWeaponActor _returnvalue))
          (Transformation|AttachComponentToComponent _output_get (Variables|Character|GetMesh) "hand_r_SwordSocket" "SnapToTarget" "SnapToTarget" "SnapToTarget" true)
          (Variables|Default|SetIsWieldingWeapon true))))))

(event Collision|EventActorBeginOverlap
  (params (OtherActor :type Actor%20Object%20Reference))
  (|CallParentFunction OtherActor) ; This node is disabled and will not be called.\nDrag off pins to build functionality.
)

(event EventUnequipWeapon
  (bind _notifyname (Animation|Montage|PlayMontage (Variables|Character|GetMesh) "/Game/Enemy/Enemy_KWANG/Animations/AM_KWANGSheathingSword_Montage.AM_KWANGSheathingSword_Montage")
    (:OnCompleted
      (Default|CallOnWeaponUnequipped :!label _label))
    (:OnInterrupted
      (goto _label))
    (:OnNotifyBegin
      (switch name _notifyname
        (:SheatSword
          (Actor|DestroyActor (Variables|Default|GetWeaponActor))
          (Variables|Default|SetIsWieldingWeapon false))))))

(event EventBeginPlay
  (|CallParentFunction)
  (Variables|/Game/Enemy/AI/AIC_Enemy_Base.AIC_Enemy_Base_C|SetHasPerception (Variables|Default|GetAIC%20Enemy%20Base) false)
  (Development|PrintString "Am oprit perceptia"))

(event EventTick
  (params (DeltaSeconds :type Float%20%28single-precision%29))
  (|CallParentFunction DeltaSeconds) ; This node is disabled and will not be called.\nDrag off pins to build functionality.
)

(event EventAttack
  (bind _returnvalue (Transformation|GetActorLocation))
  (bind _notifyname (Animation|Montage|PlayMontage (Variables|Character|GetMesh) "/Game/Enemy/Enemy_KWANG/Animations/AM_KWANGAttack_Downward_Montage.AM_KWANGAttack_Downward_Montage")
    (:then
      (Variables|/Game/DamageSystem/BPC_DamageSystem.BPC_DamageSystem_C|SetIsIntrerruptible (Variables|Default|GetBPC_DamageSystem) false))
    (:OnCompleted
      (Default|CallOnAttackEnd :!label _label)
      (Variables|/Game/DamageSystem/BPC_DamageSystem.BPC_DamageSystem_C|SetIsIntrerruptible (Variables|Default|GetBPC_DamageSystem) true))
    (:OnInterrupted
      (goto _label))
    (:OnNotifyBegin
      (switch name _notifyname
        (:Slash
          (bind (_outhit _returnvalue_2) (Collision|SphereTraceForObjects _returnvalue (+ (* (Transformation|GetActorForwardVector) 5e+02) _returnvalue) 2e+01 (Utilities|Array|MakeArray "ObjectTypeQuery3") false 0 "ForDuration"))
          (if _returnvalue_2
            (Class|BPIDamageable|TakeDamage(Message) (.HitActor (Collision|BreakHitResult _outhit)) (Utilities|Struct|MakeST_DamageInfo 3e+01 "NewEnumerator1" "NewEnumerator0" false false false true) self)))))))

(fn ConstructionScript
  (|CallParentFunction))

(fn GetMaxHealth
  (return (Variables|/Game/DamageSystem/BPC_DamageSystem.BPC_DamageSystem_C|GetMaxHealth (Variables|Default|GetBPC_DamageSystem))))

(fn GetCurrentHealth
  (return (Variables|/Game/DamageSystem/BPC_DamageSystem.BPC_DamageSystem_C|GetHealth (Variables|Default|GetBPC_DamageSystem))))